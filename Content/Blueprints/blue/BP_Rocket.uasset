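; Rocket projectile actor that flies via a ProjectileMovement component and destroys itself on overlap with another actor.
; BeginPlay runs two sequence branches that set initial and max speed, then re-apply the same values after short delays, with a debug print in one.
; Both branches converge on setting a limited lifespan.
; On overlap it spawns an emitter and a sound at its location, with no damage logic.
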(event `self.ReceiveBeginPlay`
  (bind _projectilemovement (`self.ProjectileMovement`))
  (bind _projectilemovement_2 (`self.ProjectileMovement`))
  (`|ExecutionSequence`
    (:`then_0`
      (set `ProjectileMovementComponent.InitialSpeed` 2000.0 _projectilemovement_2)
      (`KismetSystemLibrary.Delay` 0.5)
      (`KismetSystemLibrary.PrintString` "Hello")
      (set `ProjectileMovementComponent.InitialSpeed` 2000.0 _projectilemovement))
    (:`then_1`
      (set `ProjectileMovementComponent.MaxSpeed` 5000.0 _projectilemovement_2)
      (`KismetSystemLibrary.Delay` 0.5)
      (set `ProjectileMovementComponent.MaxSpeed` 5000.0 _projectilemovement)))
  (`self.SetLifeSpan` 5.0))

(event `self.ReceiveActorBeginOverlap`
  (params (OtherActor :type "Actor Object Reference"))
  (`GameplayStatics.SpawnEmitterAtLocation` null (`self.K2_GetActorLocation`) (`self.K2_GetActorRotation`))
  (`GameplayStatics.SpawnSoundAtLocation` null (`self.K2_GetActorLocation`) (struct) 1.0 1.0 0.0 null null)
  (`self.K2_DestroyActor`))

(fn `UserConstructionScript`)