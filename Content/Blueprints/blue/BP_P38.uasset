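; BP_P38 is a player-controlled P-38 plane that flies constantly forward and fires rockets.
; Pitch and Roll axes rotate it locally, scaled by RotationSpeed and delta time, while Tick feeds forward movement input scaled by Boost, raised while the Boost key is held.
; Fire spawns a BP_Rocket at the RockerSpawn transform.
; BeginPlay hands Right and Left, likely the propellers, to BPRotatingStaticMeshComponent to spin on X; RotatePropeller is an empty stub.
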(event `InputAxis|Pitch`
  (params (AxisValue :type "Float (single-precision)"))
  (`self.K2_AddActorLocalRotation` (`KismetMathLibrary.MakeRotator` 0.0 (* AxisValue (`self.RotationSpeed`) (`GameplayStatics.GetWorldDeltaSeconds`)))))

(event `InputAxis|Roll`
  (params (AxisValue :type "Float (single-precision)"))
  (`self.K2_AddActorLocalRotation` (`KismetMathLibrary.MakeRotator` (* AxisValue (`self.RotationSpeed`) (`GameplayStatics.GetWorldDeltaSeconds`)))))

(event `InputAction|Fire`
  (params (Key :type "Key Structure"))
  (:`Pressed`
    (`|SpawnActorFromClass` "/Game/Blueprints/blue/BP_Rocket.BP_Rocket_C" (`SceneComponent.K2_GetComponentToWorld` (`self.RockerSpawn`)) "Undefined" "MultiplyWithRoot" null null)))

(event `self.ReceiveTick`
  (params (DeltaSeconds :type "Float (single-precision)"))
  (`self.AddMovementInput` (`self.GetActorForwardVector`) (`self.Boost`)))

(event `InputAction|Boost`
  (params (Key :type "Key Structure"))
  (:`Pressed`
    (set `self.Boost` 1.0))
  (:`Released`
    (set `self.Boost` 0.5)))

(event `self.ReceiveBeginPlay`
  (`/Game/Blueprints/blue/BP_RotatingStaticMeshComponent.AddSceneComponent` (`self.BP_RotatingStaticMeshComponent`) (`self.Right`))
  (`/Game/Blueprints/blue/BP_RotatingStaticMeshComponent.AddSceneComponent` (`self.BP_RotatingStaticMeshComponent`) (`self.Left`))
  (set `/Game/Blueprints/blue/BP_RotatingStaticMeshComponent.Axis` (struct :`Roll` 1.0) (`self.BP_RotatingStaticMeshComponent`)))

(fn `RotatePropeller`
  (params (Where :type "SceneComponent Object Reference")))

(fn `UserConstructionScript`)