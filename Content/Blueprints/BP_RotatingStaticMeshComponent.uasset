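; BP_RotatingStaticMeshComponent continuously spins a list of registered scene components.
; AddSceneComponent appends a component to the SceneComponents array.
; Each Tick loops over that array and adds a local rotation of Axis times Speed, scaled by world delta seconds for frame-rate independent motion.
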(event `self.ReceiveTick`
  (params (DeltaSeconds :type "Float (single-precision)"))
  (for _array_element (`self.SceneComponents`)
    (`SceneComponent.K2_AddLocalRotation` _array_element (* (* (`self.Axis`) (`self.Speed`)) (`GameplayStatics.GetWorldDeltaSeconds`)) false false)))

(fn `AddSceneComponent`
  (params (RotateComponent :type "SceneComponent Object Reference"))
  (`KismetArrayLibrary.Array_Add` (`self.SceneComponents`) RotateComponent))